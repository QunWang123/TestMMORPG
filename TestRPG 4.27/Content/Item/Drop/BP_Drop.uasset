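; Dropped-item actor that players can approach, with a floating label showing its item ID.
; Sphere overlaps with the player character tell BP_MyController to add or remove the item's viewport entry by drop index.
; Each tick the label interpolates toward the player camera, using a fixed delta time rather than frame time.
; After 120 seconds it removes itself from the GameInstance's OnLineDrops, logs the expiry and destroys itself.
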(event OnComponentBeginOverlap(Sphere)
  (params (OverlappedComponent :type Primitive%20Component%20Object%20Reference) (OtherActor :type Actor%20Object%20Reference) (OtherComp :type Primitive%20Component%20Object%20Reference) (OtherBodyIndex :type Integer) (bFromSweep :type Boolean) (SweepResult :type Hit%20Result%20Structure%20%28by%20ref%29))
  (bind _itemdata (Variables|Default|GetItemData))
  (bind (_ftime _lock_index _lock_teamid _dropindex _dropid) (Utilities|Struct|BreakDROP_BASE _itemdata))
  (Utilities|Casting|CastToBP_MyCharacter OtherActor)
  (bind _asbp_my_controller (Utilities|Casting|CastToBP_MyController (Game|GetPlayerController 0)))
  (Default|AddItemtoViewport _asbp_my_controller _dropindex _dropid))

(event OnComponentEndOverlap(Sphere)
  (params (OverlappedComponent :type Primitive%20Component%20Object%20Reference) (OtherActor :type Actor%20Object%20Reference) (OtherComp :type Primitive%20Component%20Object%20Reference) (OtherBodyIndex :type Integer))
  (Utilities|Casting|CastToBP_MyCharacter OtherActor)
  (bind _asbp_my_controller (Utilities|Casting|CastToBP_MyController (Game|GetPlayerController 0)))
  (Default|RemoveItemfromViewport _asbp_my_controller (.dropindex (Utilities|Struct|BreakDROP_BASE (Variables|Default|GetItemData)))))

(event EventBeginPlay
  (bind _itemdata (Variables|Default|GetItemData))
  (bind _itemdata_2 (Variables|Default|GetItemData))
  (bind _dropindex (Utilities|Struct|BreakDROP_BASE _itemdata))
  (bind (_ftime _lock_index _lock_teamid _dropindex_2 _dropid) (Utilities|Struct|BreakDROP_BASE _itemdata_2))
  (CallFunction|SetItemText)
  (Utilities|FlowControl|Delay 1.2e+02)
  (Utilities|FlowControl|Sequence
    (:then_0
      (bind _asbp_game_instance (Utilities|Casting|CastToBP_GameInstance (Game|GetGameInstance)))
      (if (.ReturnValue (Utilities|Map|Find (Variables|/Game/GameMode/BP_GameInstance.BP_GameInstance_C|GetonLineDrops _asbp_game_instance) _dropindex))
        (Utilities|Map|Remove (Variables|/Game/GameMode/BP_GameInstance.BP_GameInstance_C|GetonLineDrops _asbp_game_instance) _dropindex)))
    (:then_1
      (Development|PrintString (Utilities|String|Append "超过120秒自动删除：" (Utilities|String|ToString(Integer) _dropindex_2) "/" (Utilities|String|ToString(Integer) _dropid)) true true "(R=0.000000,G=0.660000,B=1.000000,A=1.000000)" 333.0)
      (Actor|DestroyActor))))

(event EventTick
  (params (DeltaSeconds :type Float%20%28single-precision%29))
  (CallFunction|UpdateRotation))

(fn ConstructionScript)

(fn UpdateRotation
  (bind _textrender (Variables|Default|GetTextRender))
  (bind _asbp_my_character (Utilities|Casting|CastToBP_MyCharacter (Pawn|GetControlledPawn (Game|GetPlayerController 0))))
  (Utilities|IsValid _asbp_my_character
    (:Is%20Valid
      (Transformation|SetWorldRotation (Variables|Default|GetTextRender) (Math|Interpolation|RInterpTo (Transformation|GetWorldRotation _textrender) (Math|Rotator|FindLookatRotation (Transformation|GetWorldLocation _textrender) (Transformation|GetWorldLocation (Variables|/Script/TestRPG.MyCharacterBase|GetEMyCameraComponent _asbp_my_character))) 1.0 5.0) false false))))

(fn SetItemText
  (Rendering|Components|TextRender|SetText (Variables|Default|GetTextRender) (Utilities|Text|ToText(String) (Utilities|String|Append "Item-" (Utilities|String|ToString(Integer) (.dropid (Utilities|Struct|BreakDROP_BASE (Variables|Default|GetItemData))))))))