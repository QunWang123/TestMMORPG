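; BP_RobotView is the visual actor for a small robot monster, driven by move, skill, HP, buff and death command callbacks.
; Move commands line-trace a ground height, then Tick interpolates yaw and steps the actor there, speeding up when far away.
; Skills face the lock target and play montages by robot and skill ID.
; A camera-facing nameplate shows HP and damage; buff actors attach by ID and are cleared on death.
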(event Custom|Event_PlayerSkill
  (params (EventCount :type Integer))
  (Utilities|MacroPlaySkill EventCount))

(event EventBeginPlay
  (bind _robotdata (Variables|Default|Getrobotdata))
  (bind (_robotindex _id _dir _hp _grid _pos _nick) (Utilities|Struct|BreakROBOT_BASE _robotdata))
  (bind _asnick_ui (Utilities|Casting|CastToNickUI (UserInterface|GetUserWidgetObject (Variables|Default|GetNick))))
  (bind _output_get (Variables|Default|SetNickUI _asnick_ui))
  (Default|SetNick _output_get (Utilities|String|Append _nick "-" (Utilities|String|ToString(Integer) _robotindex)))
  (CallFunction|SetCurHP (Math|Conversions|ToFloat(Integer) _hp)))

(event EventTick
  (params (DeltaSeconds :type Float%20%28single-precision%29))
  (CallFunction|UpdateMove DeltaSeconds)
  (CallFunction|UpdateNickUI))

(fn ConstructionScript)

(fn UpdateNickUI
  (bind _nick (Variables|Default|GetNick))
  (bind _asbp_my_character (Utilities|Casting|CastToBP_MyCharacter (Pawn|GetControlledPawn (Game|GetPlayerController 0))))
  (Utilities|IsValid _asbp_my_character
    (:Is%20Valid
      (Utilities|IsValid _nick
        (:Is%20Valid
          (Transformation|SetWorldRotation (Variables|Default|GetNick) (Math|Interpolation|RInterpTo (Transformation|GetWorldRotation _nick) (Math|Rotator|FindLookatRotation (Transformation|GetWorldLocation _nick) (Transformation|GetWorldLocation (Variables|/Script/TestRPG.MyCharacterBase|GetEMyCameraComponent _asbp_my_character))) 1.0 5.0) false false))))))

(fn SetAnimHP
  (params (CurHP :type Integer))
  (bind _asthird_person_anim_bp (Utilities|Casting|CastToThirdPerson_AnimBP (Components|SkeletalMesh|GetAnimInstance (Variables|Character|GetMesh))))
  (Variables|/Game/Robot/Monster/Mannequin/Animations/ThirdPerson_AnimBP.ThirdPerson_AnimBP_C|SetCurhp _asthird_person_anim_bp CurHP))

(fn SetCurHP
  (params (Value :type Float%20%28single-precision%29))
  (bind _nickui (Variables|Default|GetNickUI))
  (Utilities|IsValid _nickui
    (:Is%20Valid
      (Default|SetCurHP _nickui (/ Value (Math|Conversions|ToFloat(Integer) (.maxhp (Utilities|Struct|BreakROBOT_BASE (Variables|Default|Getrobotdata)))))))))

(fn OnSkillCommandHP
  (params (curhp :type Integer) (atk :type Integer))
  (Utilities|FlowControl|Sequence
    (:then_0
      (if (!= atk -99)
        (Default|ShowDamage (Variables|Default|GetNickUI) true atk)))
    (:then_1
      (CallFunction|SetCurHP (Math|Conversions|ToFloat(Integer) curhp))
      (return false))))

(fn OnCommandDead
  (Utilities|FlowControl|Sequence
    (:then_0
      (CallFunction|SetAnimHP))
    (:then_1
      (Components|DestroyComponent (Variables|Default|GetNick)))
    (:then_2
      (bind _values (Utilities|Map|Values (Variables|Default|GetBuff_Run)))
      (for _array_element _values
        (Actor|DestroyActor _array_element))
      (Utilities|Map|Clear (Variables|Default|GetBuff_Run)))
    (:then_3
      (return false))))

(fn UpdateMove
  (params (Value :type Float%20%28single-precision%29))
  (LocalVariables|SetFrameDeltaTime Value)
  (if (Variables|Default|GetisMoveTargetPos)
    (Utilities|FlowControl|Sequence
      (:then_0
        (Transformation|SetActorRotation (Math|Interpolation|RInterpTo (Math|Rotator|MakeRotator 0.0 0.0 (.yaw (Transformation|GetActorRotation))) (Math|Rotator|MakeRotator 0.0 0.0 (Variables|Default|GetTargetFace)) (* 16 (LocalVariables|GetFrameDeltaTime)) 0.0)))
      (:then_1
        (LocalVariables|SetLocalPos (Math|Vector|Normalize (- (Variables|Default|GetTargetPos) (Transformation|GetActorLocation)))))
      (:then_2
        (bind _output_get (LocalVariables|SetLocalDistance (Math|Vector|Distance(Vector) (Transformation|GetActorLocation) (Variables|Default|GetTargetPos))))
        (if (> _output_get 2e+01)
          (if (>= (LocalVariables|GetLocalDistance) 2.5e+02)
            ;[1 1 1] 距离差的太远了
            (LocalVariables|SetLocalCurSpeed (* (Variables|/Script/Engine.CharacterMovementComponent|GetMaxWalkSpeed (Variables|Character|GetCharacterMovement)) 1.5))
            (else
              (LocalVariables|SetLocalCurSpeed (Variables|Default|GetTargetSpeed))))
          (Transformation|SetActorLocation (+ (Transformation|GetActorLocation) (* (LocalVariables|GetLocalPos) (* (LocalVariables|GetLocalCurSpeed) (LocalVariables|GetFrameDeltaTime)))) false false)
          (else
            (Variables|Default|SetTargetSpeed 0.0)
            (Variables|Default|SetisMoveTargetPos false)
            (Class|RobotBase|InitEventing (.robotindex (Utilities|Struct|BreakROBOT_BASE (Variables|Default|Getrobotdata))))))))))

(fn OnCommandMove
  (params (pos :type Vector :default "0, 0, 0") (num :type Integer))
  (bind _pos (CallFunction|GetMainLocation))
  (Variables|Default|SetTargetPos (Math|Vector|MakeVector (.x pos) (.y pos) 0.0))
  (bind _outhit (Collision|LineTraceForObjects (Math|Vector|MakeVector (.x (Variables|Default|GetTargetPos)) (.y (Variables|Default|GetTargetPos)) (+ (.z _pos) -1e+03)) (Math|Vector|MakeVector (.x (Variables|Default|GetTargetPos)) (.y (Variables|Default|GetTargetPos)) (+ (.z _pos) 1e+03)) (Utilities|Array|MakeArray "ObjectTypeQuery1" "ObjectTypeQuery2") false 0 "None"))
  (Variables|Default|SetTargetPos (Math|Vector|MakeVector (.x (Variables|Default|GetTargetPos)) (.y (Variables|Default|GetTargetPos)) (+ (.Z (Math|Vector|BreakVector (.Location (Collision|BreakHitResult _outhit)))) 1e+02)))
  (Variables|Default|SetTargetFace (.yaw (Math|Rotator|FindLookatRotation (Transformation|GetActorLocation) (Variables|Default|GetTargetPos))))
  (Variables|Default|SetTargetSpeed (Variables|/Script/Engine.CharacterMovementComponent|GetMaxWalkSpeed (Variables|Character|GetCharacterMovement)))
  (Variables|Default|SetisMoveTargetPos true))

(fn GetMainLocation
  (bind _asbp_my_character (Utilities|Casting|CastToBP_MyCharacter (Pawn|GetControlledPawn (Game|GetPlayerController 0)))
    (:then
      (return (Transformation|GetActorLocation _asbp_my_character)))
    (:CastFailed
      (return (Class|BlueprintFunction|GetMapLeftPos)))))

(fn OnBuffCommandPlay
  (params (id :type Integer) (runningtime :type Integer))
  (LocalVariables|SetLocalBuffID id)
  (LocalVariables|SetLocalRunTime runningtime)
  (LocalVariables|SetLocalBuff (.Value (Utilities|Map|Find (Variables|Default|GetBuff_Run) (LocalVariables|GetLocalBuffID))))
  (switch int (LocalVariables|GetLocalRunTime)
    (:Default
      (Utilities|IsValid (LocalVariables|GetLocalBuff)
        (:Is%20Not%20Valid
          (bind _returnvalue (Game|SpawnActorfromClass "/Game/BuffandSkill/Role_Buff.Role_Buff_C" (Math|Transform|MakeTransform "0, 0, 0" "0, 0, 0" "1,1,1") "Undefined" self 0))
          (bind _output_get (LocalVariables|SetLocalBuff _returnvalue))
          (Transformation|AttachActorToActor _output_get self "None" "KeepRelative" "KeepRelative" "KeepRelative" true)
          (Default|SetBuff (LocalVariables|GetLocalBuff) (LocalVariables|Getlocalbuffid))
          (Utilities|Map|Add (Variables|Default|Getbuff_run) (LocalVariables|Getlocalbuffid) (LocalVariables|GetLocalBuff)))))
    (:0
      (Utilities|Map|Remove (Variables|Default|GetBuff_Run) (LocalVariables|GetLocalBuffID))
      (Actor|DestroyActor (LocalVariables|GetLocalBuff)))))

(fn OnSkillCommandPlay
  (params (num :type Integer))
  (CallFunction|EventPlayerSkill num)
  (return true))