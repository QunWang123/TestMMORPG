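; Game mode that prunes other online players' characters around the local player, alongside starting heartbeat timing and running the app update each tick.
; About every 0.3 seconds it scans all OtherCharacter actors, testing each against the local character's nine-cell grid area and its own heartbeat timeout.
; Failing either check removes the user from the game instance's OnLineUsers, prints a removal message, and destroys the actor.
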(event EventBeginPlay
  (Class|BlueprintFunction|InitHeartTime)
  (Variables|Default|SetCheck_temptime (Utilities|Time|GetTimeSeconds)))

(event EventTick
  (params (DeltaSeconds :type Float%20%28single-precision%29))
  (Class|BlueprintFunction|AppUpdate)
  (CallFunction|UpdataOnlinesRect))

(fn ConstructionScript)

(fn UpdataOnlinesRect
  (if (> (- (Utilities|Time|GetTimeSeconds) (Variables|Default|GetCheck_temptime)) 0.3)
    (Variables|Default|SetCheck_temptime (Utilities|Time|GetTimeSeconds))
    (bind _asbp_game_instance (Utilities|Casting|CastToBP_GameInstance (Game|GetGameInstance)))
    (LocalVariables|SetLocalGameInstance _asbp_game_instance)
    (bind _asbp_my_character (Utilities|Casting|CastToBP_MyCharacter (Pawn|GetControlledPawn (Game|GetPlayerController 0))))
    (LocalVariables|SetLocalMyCharacter _asbp_my_character)
    (bind _outactors (Actor|GetAllActorsOfClass "/Game/Character/OtherCharacter/OtherCharacter.OtherCharacter_C"))
    (for _array_element _outactors
      (LocalVariables|SetLocalOther _array_element)
      (LocalVariables|SetLocalIsDelete false)
      (Utilities|FlowControl|Sequence
        (:then_0
          (bind _returnvalue (Class|MyCharacterBase|IsMainRect (LocalVariables|GetLocalMyCharacter) (Transformation|GetActorLocation (LocalVariables|GetLocalOther))))
          (if (not _returnvalue)
            (Utilities|FlowControl|Sequence :!label _label
              (:then_0
                (if (.ReturnValue (Utilities|Map|Find (Variables|/Game/GameMode/BP_GameInstance.BP_GameInstance_C|GetonLineUsers (LocalVariables|GetLocalGameInstance)) (.userindex (Utilities|Struct|BreakOTHER_ROLE_BASE (Variables|/Game/Character/OtherCharacter/OtherCharacter.OtherCharacter_C|GetOtherUserData (LocalVariables|GetLocalOther))))))
                  (Utilities|Map|Remove (Variables|/Game/GameMode/BP_GameInstance.BP_GameInstance_C|GetonLineUsers (LocalVariables|GetLocalGameInstance)) (.userindex (Utilities|Struct|BreakOTHER_ROLE_BASE (Variables|/Game/Character/OtherCharacter/OtherCharacter.OtherCharacter_C|GetOtherUserData (LocalVariables|GetLocalOther)))))
                  (Development|PrintString (Utilities|String|Append (.nick (Utilities|Struct|BreakOTHER_ROLE_BASE (Variables|/Game/Character/OtherCharacter/OtherCharacter.OtherCharacter_C|GetOtherUserData (LocalVariables|GetLocalOther)))) "不在九宫格范围内，移除" (Utilities|String|ToString(Integer) (.userindex (Utilities|Struct|BreakOTHER_ROLE_BASE (Variables|/Game/Character/OtherCharacter/OtherCharacter.OtherCharacter_C|GetOtherUserData (LocalVariables|GetLocalOther))))) "！"))
                  (LocalVariables|SetLocalIsDelete true)))
              (:then_1
                (Actor|DestroyActor (LocalVariables|GetLocalOther))))))
        (:then_1
          (if (not (LocalVariables|GetLocalIsDelete))
            (Utilities|IsValid (LocalVariables|GetLocalOther)
              (:Is%20Valid
                (bind _ish (Default|IsOutHeartTime (LocalVariables|GetLocalOther)))
                (if _ish
                  (goto _label))))))))))