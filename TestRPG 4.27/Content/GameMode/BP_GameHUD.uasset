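; Game HUD that creates the main UI widget and manages the player's bag/combat inventory widget.
; Toggling the bag switches cursor and input mode; if no bag exists, it sends bag and combat data requests instead.
; The update-all functions lazily create the bag widget and refresh its grids.
; Other functions forward slot and attack updates to the bag, and HP, damage, log, chat and item-slot calls to the main UI.
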(event EventBeginPlay
  (bind _returnvalue (UserInterface|CreateWidget "/Game/UI/GameUI/MainUI.MainUI_C"))
  (bind _output_get (Variables|Default|SetMainUI _returnvalue))
  (UserInterface|Viewport|AddtoViewport _output_get 0)
  (Default|UpdataHeadInfo (Variables|Default|GetMainUI)))

(event Collision|EventActorBeginOverlap
  (params (OtherActor :type Actor%20Object%20Reference)))

(event EventTick
  (params (DeltaSeconds :type Float%20%28single-precision%29)))

(fn ConstructionScript)

(fn ShowBagWidget
  (bind _returnvalue (Game|GetPlayerController 0))
  (Utilities|IsValid (Variables|Default|GetBagWidget)
    (:Is%20Valid
      (switch Utilities|FlowControl|Switch|SwitchonESlateVisibility (Widget|GetVisibility (Variables|Default|GetBagWidget))
        (:Visible
          (Widget|SetVisibility (Variables|Default|GetBagWidget) "Hidden" :!label _label)
          (Variables|/Script/Engine.PlayerController|SetbShowMouseCursor _returnvalue false)
          (bind _asbp_my_controller (Utilities|Casting|CastToBP_MyController _returnvalue))
          (Input|SetInputModeGameOnly _asbp_my_controller))
        (:Collapsed
          (goto _label))
        (:Hidden
          (Widget|SetVisibility (Variables|Default|GetBagWidget) "Visible")
          (Variables|/Script/Engine.PlayerController|SetbShowMouseCursor _returnvalue true)
          (bind _asbp_my_controller_2 (Utilities|Casting|CastToBP_MyController _returnvalue))
          (Input|SetInputModeUIOnly _asbp_my_controller_2 (Variables|Default|GetBagWidget) "DoNotLock")
          (Class|UIBag|UpdateCombatHeadInfo (Variables|Default|GetBagWidget)))
        (:HitTestInvisible
          (goto _label))
        (:SelfHitTestInvisible
          (goto _label))))
    (:Is%20Not%20Valid
      (Utilities|FlowControl|Sequence
        (:then_0
          (Class|BlueprintFunction|SendGetCombat (.userindex (Utilities|Struct|BreakUSER_ROLE_BASE (Class|BlueprintFunction|MyUserData))))
          (Class|BlueprintFunction|SendGetBag))
        (:then_1
          (return))))))

(fn UpdateAllBagGrid
  (bind _returnvalue (Game|GetPlayerController 0))
  (Utilities|IsValid (Variables|Default|GetBagWidget)
    (:Is%20Valid
      (Input|SetInputModeUIOnly _returnvalue (Variables|Default|GetBagWidget) "DoNotLock"))
    (:Is%20Not%20Valid
      (bind _returnvalue_2 (UserInterface|CreateWidget "/Game/UI/Bag/BPUI_Bag.BPUI_Bag_C"))
      (bind _output_get (Variables|Default|SetBagWidget _returnvalue_2))
      (UserInterface|Viewport|AddtoViewport _output_get 0)
      (Variables|/Script/Engine.PlayerController|SetbShowMouseCursor _returnvalue true)))
  (Class|UIBag|UpdateAllBagInfo (Variables|Default|GetBagWidget))
  (Bag|UpdateAllCombatGrid))

(fn UpdateAllCombatGrid
  (bind _returnvalue (Game|GetPlayerController 0))
  (Utilities|IsValid (Variables|Default|GetBagWidget)
    (:Is%20Valid
      (Class|UIBag|UpdateAllCombatInfo (Variables|Default|GetBagWidget))
      (Class|UIBag|UpdateCombatHeadInfo (Variables|Default|GetBagWidget)))
    (:Is%20Not%20Valid
      (bind _returnvalue_2 (UserInterface|CreateWidget "/Game/UI/Bag/BPUI_Bag.BPUI_Bag_C"))
      (bind _output_get (Variables|Default|SetBagWidget _returnvalue_2))
      (UserInterface|Viewport|AddtoViewport _output_get 0)
      (Variables|/Script/Engine.PlayerController|SetbShowMouseCursor _returnvalue true)
      (Input|SetInputModeUIOnly _returnvalue (Variables|Default|GetBagWidget) "DoNotLock"))))

(fn UpdateBagSpecifyGrid
  (params (index :type Byte))
  (bind _bagwidget (Variables|Default|GetBagWidget))
  (Utilities|IsValid _bagwidget
    (:Is%20Valid
      (Class|UIBag|UpdateBagSpecifyGrid _bagwidget index))))

(fn UpdateBagSpecifyGridNum
  (params (Index :type Byte))
  (bind _bagwidget (Variables|Default|GetBagWidget))
  (Utilities|IsValid _bagwidget
    (:Is%20Valid
      (Class|UIBag|UpdateBagSpecifyGridNum _bagwidget Index))))

(fn UpdateCombatSpecifyGrid
  (params (Index :type Byte))
  (bind _bagwidget (Variables|Default|GetBagWidget))
  (Utilities|IsValid _bagwidget
    (:Is%20Valid
      (Class|UIBag|UpdateCombatSpecifyGrid _bagwidget Index))))

(fn UpdateCombatAtk
  (bind _bagwidget (Variables|Default|GetBagWidget))
  (Utilities|IsValid _bagwidget
    (:Is%20Valid
      (Class|UIBag|UpdateCombatAtk _bagwidget))))

(fn UpdateMainCharacterHP
  (params (CurHP :type Float%20%28single-precision%29) (atk :type Integer))
  (bind _mainui (Variables|Default|GetMainUI))
  (Default|SetCurHP _mainui CurHP)
  (if (!= atk 0)
    (Default|ShowDamage _mainui true atk)))

(fn LogMsg
  (params (Msg :type String))
  (Default|LogMsg (Variables|Default|GetMainUI) Msg))

(fn AddChatText
  (params (InText :type String))
  (Default|AddChatText (Variables|Default|GetMainUI) InText))

(fn ShowChatUI
  (params (InVisibility :type ESlateVisibility%20Enum :default "Visible"))
  (Default|ShowChatUI (Variables|Default|GetMainUI) InVisibility))

(fn AddItemSlot
  (params (ItemIndex :type Integer) (ItemID :type Integer))
  (Default|AddItemSlot (Variables|Default|GetMainUI) ItemIndex ItemID))

(fn RemoveItemSlot
  (params (ItemIndex :type Integer))
  (Default|RemoveItemSlot (Variables|Default|GetMainUI) ItemIndex))