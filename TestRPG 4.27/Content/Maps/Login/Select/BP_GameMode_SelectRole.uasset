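; Game mode for the role selection map, managing the role select and role creation screens and ticking the app update.
; BeginPlay enables UI-only mouse input and creates both widgets, with SetUIVisible toggling between them and reinitializing the creation screen when shown.
; OnSelectRoleCommand branches on command codes for entering, creating, deleting and starting, refreshing the UI or logging errors through the GameInstance.
; A successful start opens the level from the role's saved map ID.
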(event EventBeginPlay
  (bind _returnvalue (Game|GetPlayerController 0))
  (Variables|/Script/Engine.PlayerController|SetbShowMouseCursor _returnvalue true)
  (Input|SetInputModeUIOnly _returnvalue (Variables|Default|GetSelect_UI) "DoNotLock")
  (Utilities|FlowControl|Sequence
    (:then_0
      (bind _returnvalue_2 (UserInterface|CreateWidget "/Game/UI/SelectUI.SelectUI_C"))
      (bind _output_get (Variables|Default|SetSelect_UI _returnvalue_2))
      (UserInterface|Viewport|AddtoViewport _output_get 1))
    (:then_1
      (bind _returnvalue_3 (UserInterface|CreateWidget "/Game/UI/CreateRoleUI.CreateRoleUI_C"))
      (bind _output_get_2 (Variables|Default|SetCreate_UI _returnvalue_3))
      (UserInterface|Viewport|AddtoViewport _output_get_2 0))
    (:then_2
      (CallFunction|SetUIVisible true))))

(event EventTick
  (params (DeltaSeconds :type Float%20%28single-precision%29))
  (Class|BlueprintFunction|AppUpdate))

(fn ConstructionScript)

(fn SetUIVisible
  (params (IsVisible :type Boolean))
  (if IsVisible
    (Widget|SetVisibility (Variables|Default|GetSelect_UI) "Visible")
    (Widget|SetVisibility (Variables|Default|GetCreate_UI) "Hidden")
    (else
      (Widget|SetVisibility (Variables|Default|GetSelect_UI) "Hidden")
      (Widget|SetVisibility (Variables|Default|GetCreate_UI) "Visible")
      (Default|SetInit (Variables|Default|GetCreate_UI)))))

(fn OnSelectRoleCommand
  (params (cmd :type Integer) (childcmd :type Integer) (indexrole :type Byte))
  (bind _returnvalue (Class|BlueprintFunction|MyUserData))
  (bind _select_ui (Variables|Default|GetSelect_UI))
  (bind _select_ui_2 (Variables|Default|GetSelect_UI))
  (bind (_select_roleindex _memid _userindex _rolebase _base) (Utilities|Struct|BreakUSER_ROLE_BASE _returnvalue))
  (bind (_exp _econ _status _life) (Utilities|Struct|BreakROLE_BASE _base))
  (bind (_level _currexp) (Utilities|Struct|BreakROLE_BASE_EXP _exp))
  (bind _mapid (Utilities|Struct|BreakROLE_BASE_STATUS _status))
  (bind (_hp _mp) (Utilities|Struct|BreakROLE_BASE_LIFE _life))
  (LocalVariables|Setlocalcmd (Utilities|String|ToString(Integer) cmd))
  (LocalVariables|Setlocalchildcmd childcmd)
  (LocalVariables|Setlocalroleindex indexrole)
  (Utilities|FlowControl|Sequence
    (:then_0
      (bind _asbp_game_instance (Utilities|Casting|CastToBP_GameInstance (Game|GetGameInstance)))
      (LocalVariables|Setlocalgameinstance _asbp_game_instance))
    (:then_1
      (switch string (LocalVariables|Getlocalcmd)
        (:200
          (if (== (LocalVariables|Getlocalchildcmd) 0)
            (Default|UpdaErrorInfo (LocalVariables|Getlocalgameinstance) (Math|Conversions|ToInteger(Byte) (LocalVariables|Getlocalcmd)) (LocalVariables|Getlocalchildcmd) "进入游戏成功！")
            (else
              (bind _returnvalue_2 (Default|UpdaErrorInfo (LocalVariables|Getlocalgameinstance) (Math|Conversions|ToInteger(Byte) (LocalVariables|Getlocalcmd)) (LocalVariables|Getlocalchildcmd) "开始游戏失败！"))
              (Default|LogMessage (Variables|Default|GetSelect_UI) _returnvalue_2))))
        (:300
          (if (== (LocalVariables|Getlocalchildcmd) 0)
            (Default|SetRoleIndex _select_ui (LocalVariables|Getlocalroleindex))
            (CallFunction|SetUIVisible true)
            (Default|UpdataRoleInfo _select_ui)
            (Default|LogMessage _select_ui "创建成功！")
            (else
              (bind _returnvalue_3 (Default|UpdaErrorInfo (LocalVariables|Getlocalgameinstance) (Math|Conversions|ToInteger(Byte) (LocalVariables|Getlocalcmd)) (LocalVariables|Getlocalchildcmd) "创建失败！"))
              (Default|LogMessage (Variables|Default|GetCreate_UI) _returnvalue_3))))
        (:400
          (if (== (LocalVariables|Getlocalchildcmd) 0)
            (Default|LogMessage _select_ui_2 "删除成功！")
            (Default|SetDefaultRoleIndex _select_ui_2)
            (Default|UpdataRoleInfo _select_ui_2)
            (else
              (bind _returnvalue_4 (Default|UpdaErrorInfo (LocalVariables|Getlocalgameinstance) (Math|Conversions|ToInteger(Byte) (LocalVariables|Getlocalcmd)) (LocalVariables|Getlocalchildcmd) "删除失败！"))
              (Default|LogMessage (Variables|Default|GetSelect_UI) _returnvalue_4))))
        (:500
          (if (== (LocalVariables|Getlocalchildcmd) 0)
            (bind _returnvalue_5 (Class|BlueprintFunction|GetMapName _mapid))
            (Game|OpenLevel(byName) (Utilities|String|StringToName _returnvalue_5))
            (Development|PrintString (Utilities|String|Append "角色数据：" (Utilities|String|ToString(Byte) _select_roleindex) "/" (.nick (Utilities|Struct|BreakUSER_MEMBER_ROLE _rolebase)) "/" (Utilities|String|ToString(Integer) _level) "/" (Utilities|String|ToString(Integer) _currexp) "/" (Utilities|String|ToString(Integer) _mapid) "/" (Utilities|String|ToString(Integer) _hp) "/" (Utilities|String|ToString(Integer) _mp)) true true "(R=0.091947,G=1.000000,B=0.082122,A=1.000000)" 6e+01)
            (else
              (bind _returnvalue_6 (Default|UpdaErrorInfo (LocalVariables|Getlocalgameinstance) (Math|Conversions|ToInteger(Byte) (LocalVariables|Getlocalcmd)) (LocalVariables|Getlocalchildcmd) "开始游戏失败！"))
              (Default|LogMessage (Variables|Default|GetSelect_UI) _returnvalue_6))))))))