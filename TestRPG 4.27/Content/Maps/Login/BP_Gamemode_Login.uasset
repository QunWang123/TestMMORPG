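; Login-map game mode that runs the client's login, registration and game-entry flow.
; BeginPlay initializes the network client through MyGameInstance and shows LoginUI with the mouse cursor, while Tick calls AppUpdate.
; OnLoginCommand handles server replies by command code, logging results or game-instance error text to the UI, and opens ThirdPersonExampleMap on game entry.
; SetUIVisiable switches the UI only when connected and already logged in, distinguishing gate-server from login-server connection.
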(event EventBeginPlay
  ;[1 1 1] 开启客户端
  (bind _asmy_game_instance (Utilities|Casting|CastToMyGameInstance (Game|GetGameInstance)))
  (Class|MyGameInstance|AppInitGameInstance _asmy_game_instance)
  (bind _returnvalue (UserInterface|CreateWidget "/Game/UI/LoginUI.LoginUI_C"))
  (bind _output_get (Variables|Default|SetLogin_UI _returnvalue))
  (UserInterface|Viewport|AddtoViewport _output_get 0)
  (Variables|/Script/Engine.PlayerController|SetbShowMouseCursor (Game|GetPlayerController 0) true))

(event EventTick
  (params (DeltaSeconds :type Float%20%28single-precision%29))
  (Class|BlueprintFunction|AppUpdate))

(fn ConstructionScript)

(fn OnLoginCommand
  (params (cmd :type Integer) (childcmd :type Integer))
  ;[1 1 1] UI发送登录、注册请求后，收到回复就走这里
  (LocalVariables|Setlocalcmd (Utilities|String|ToString(Integer) cmd))
  (LocalVariables|Setlocalchildcmd childcmd)
  (Utilities|FlowControl|Sequence
    (:then_0
      (bind _asbp_game_instance (Utilities|Casting|CastToBP_GameInstance (Game|GetGameInstance))
        (:then
          (LocalVariables|Setlocalgameinstance _asbp_game_instance))
        (:CastFailed
          (return))))
    (:then_1
      (switch string (LocalVariables|Getlocalcmd)
        (:10
          (if (== (LocalVariables|Getlocalchildcmd) 0)
            (Default|LogMessage (Variables|Default|GetLogin_UI) "登录成功，选择服务器")
            (Variables|Default|Setislogin true)
            (else
              (bind _returnvalue (Default|UpdaErrorInfo (LocalVariables|Getlocalgameinstance) (Math|Conversions|ToInteger(Byte) (LocalVariables|Getlocalcmd)) (LocalVariables|Getlocalchildcmd) "登录失败！"))
              (Default|LogMessage (Variables|Default|GetLogin_UI) _returnvalue)
              (Variables|Default|Setislogin false))))
        (:20
          (if (== (LocalVariables|Getlocalchildcmd) 0)
            (Default|LogMessage (Variables|Default|GetLogin_UI) "注册成功！")
            (else
              (bind _returnvalue_2 (Default|UpdaErrorInfo (LocalVariables|Getlocalgameinstance) (Math|Conversions|ToInteger(Byte) (LocalVariables|Getlocalcmd)) (LocalVariables|Getlocalchildcmd) "注册失败！"))
              (Default|LogMessage (Variables|Default|GetLogin_UI) _returnvalue_2))))
        (:100
          (if (== (LocalVariables|Getlocalchildcmd) 0)
            (Default|LogMessage (Variables|Default|GetLogin_UI) "登录游戏成功！")
            (Game|OpenLevel(byName) "ThirdPersonExampleMap")
            (else
              (bind _returnvalue_3 (Default|UpdaErrorInfo (LocalVariables|Getlocalgameinstance) (Math|Conversions|ToInteger(Byte) (LocalVariables|Getlocalcmd)) (LocalVariables|Getlocalchildcmd) "登录游戏失败！"))
              (Default|LogMessage (Variables|Default|GetLogin_UI) _returnvalue_3))))))))

(fn SetUIVisiable
  (params (IsConnect :type Boolean))
  (if IsConnect
    ;[1 1 1] 一开始连接loginserver的时候，由于没有登录，所以会走false,连上gateserver之后就true了
    (if (Variables|Default|Getislogin)
      (Default|SetVisiable (Variables|Default|GetLogin_UI) 1))))