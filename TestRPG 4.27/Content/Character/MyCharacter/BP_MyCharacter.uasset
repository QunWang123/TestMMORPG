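; BP_MyCharacter is the locally controlled player character of a networked game, spawned from stored user data.
; Tick sends throttled move updates with an obstacle-checked predicted target position.
; Skill use sets a lock target and validates before sending, auto-following via the controller when needed.
; Command handlers apply server results: position correction, skill montages, buff actors, cooldown UI, death and reborn; the HP update is unwired.
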(event Custom|Event_PlaySkill
  (Utilities|EventPlaySkill))

(event Custom|Event_PlayDead
  (Utilities|EventPlayDead))

(event EventBeginPlay
  (if (Pawn|IsLocallyControlled)
    (Utilities|FlowControl|Sequence
      (:then_0
        (CallFunction|SetGameInstance)
        (Class|MyCharacterBase|SetCharacter self)
        (bind _returnvalue (UserInterface|CreateWidget "/Game/UI/GameUI/SkillUI.SkillUI_C"))
        (bind _output_get (Variables|Default|SetSkillUI _returnvalue))
        (UserInterface|Viewport|AddtoViewport _output_get 0))
      (:then_1
        (Class|BlueprintFunction|SendEntryWorld))
      (:then_2
        (Variables|Default|Setuserdata (Class|BlueprintFunction|MyUserData))
        (CallFunction|UpdatePos)
        (CallFunction|ChangeWeapon)
        (CallFunction|OnSkillCommandHP (.hp (Utilities|Struct|BreakROLE_BASE_LIFE (.life (Utilities|Struct|BreakROLE_BASE (.base (Utilities|Struct|BreakUSER_ROLE_BASE (Variables|Default|Getuserdata)))))))))
      (:then_3
        (bind _asbp_my_controller (Utilities|Casting|CastToBP_MyController (Game|GetPlayerController 0)))
        (Variables|Default|SetMyPlayerController _asbp_my_controller)))))

(event EventTick
  (params (DeltaSeconds :type Float%20%28single-precision%29))
  (if (Pawn|IsLocallyControlled)
    (Variables|Move|SetSpeed (Math|Vector|VectorLength (Transformation|GetVelocity)))
    (CallFunction|UpdataSyncedMove)
    (CallFunction|UpdateFollowATK)))

(event Input|KeyboardEvents|Q
  (params (Key :type Key%20Structure))
  (:Pressed
    (Development|ExecuteConsoleCommand "Quit" 0)))

(event Input|KeyboardEvents|1
  (params (Key :type Key%20Structure))
  (:Released
    (bind _output_get (Variables|Default|SetLocalSkillIndex 6))
    (Class|MyCharacterBase|SendSkill _output_get)))

(event Input|KeyboardEvents|2
  (params (Key :type Key%20Structure))
  (:Released
    (bind _output_get (Variables|Default|SetLocalSkillIndex 7))
    (Class|MyCharacterBase|SendSkill _output_get)))

(fn ConstructionScript)

(fn SetGameInstance
  (Utilities|IsValid (Variables|Default|GetMyGameInstance)
    (:Is%20Not%20Valid
      (bind _asbp_game_instance (Utilities|Casting|CastToBP_GameInstance (Game|GetGameInstance)))
      (Variables|Default|SetMyGameInstance _asbp_game_instance))))

(fn UpdatePos
  (bind _returnvalue (Class|BlueprintFunction|GetMapLeftPos))
  (bind _userdata (Variables|Default|Getuserdata))
  (bind _base (Utilities|Struct|BreakUSER_ROLE_BASE _userdata))
  (bind _status (Utilities|Struct|BreakROLE_BASE _base))
  (bind (_state _face _mapid _pos) (Utilities|Struct|BreakROLE_BASE_STATUS _status))
  (LocalVariables|SetLocalPos _pos)
  (LocalVariables|SetLocalFace (/ (Math|Conversions|ToFloat(Integer) _face) 1e+02))
  (if (== (.z (LocalVariables|GetLocalPos)) 0)
    (bind _outhit (Collision|LineTraceForObjects (Math|Vector|MakeVector (Math|Conversions|ToFloat(Integer) (.x (LocalVariables|GetLocalPos))) (Math|Conversions|ToFloat(Integer) (.y (LocalVariables|GetLocalPos))) (+ (.z _returnvalue) 3e+03)) (Math|Vector|MakeVector (Math|Conversions|ToFloat(Integer) (.x (LocalVariables|GetLocalPos))) (Math|Conversions|ToFloat(Integer) (.y (LocalVariables|GetLocalPos))) (+ (.z _returnvalue) -3e+03)) (Utilities|Array|MakeArray "ObjectTypeQuery1" "ObjectTypeQuery2") false 0 "Persistent"))
    (Transformation|SetActorLocationAndRotation (Math|Vector|MakeVector (Math|Conversions|ToFloat(Integer) (.x (LocalVariables|GetLocalPos))) (Math|Conversions|ToFloat(Integer) (.y (LocalVariables|GetLocalPos))) (+ (.Z (Math|Vector|BreakVector (.Location (Collision|BreakHitResult _outhit)))) 2.5e+02)) (Math|Rotator|MakeRotator 0.0 0.0 (LocalVariables|GetLocalFace)))
    (else
      (Transformation|SetActorLocationAndRotation (Math|Vector|MakeVector (Math|Conversions|ToFloat(Integer) (.x (Utilities|Struct|BreakS_VECTOR (LocalVariables|GetLocalPos)))) (Math|Conversions|ToFloat(Integer) (.y (Utilities|Struct|BreakS_VECTOR (LocalVariables|GetLocalPos)))) (Math|Conversions|ToFloat(Integer) (.z (Utilities|Struct|BreakS_VECTOR (LocalVariables|GetLocalPos))))) (Math|Rotator|MakeRotator 0.0 0.0 (LocalVariables|GetLocalFace))))))

(fn ChangeWeapon
  ;[1 1 1] 设置武器
  (switch string (Utilities|String|ToString(Byte) (.job (Utilities|Struct|BreakUSER_MEMBER_ROLE (.rolebase (Utilities|Struct|BreakUSER_ROLE_BASE (Variables|Default|Getuserdata))))))))

(fn UpdataSyncedMove
  (if (Class|BlueprintFunction|IsLogin)
    (Utilities|FlowControl|Sequence
      (:then_0
        (if (<= (Variables|Move|GetSpeed) 0.0)
          (LocalVariables|Setlocalstate 0)
          (else
            (LocalVariables|Setlocalstate 1)))
        ;[1 1 1] 记录speed=0时的最后时刻
        (if (== (Variables|Move|GetsyncedState) 0)
          (Variables|Move|SetsyncedTimeTemp (Utilities|Time|GetTimeSeconds))))
      (:then_1
        ;[1 1 1] 刚起步或刚停下即状态切换
        (if (!= (Variables|Move|GetsyncedState) (LocalVariables|Getlocalstate))
          (CallFunction|SendSyncedMove 0 (LocalVariables|Getlocalstate))
          (return)))
      (:then_2
        (if (> (Math|Float|Absolute(Float) (- (.yaw (Transformation|GetActorRotation)) (Variables|Move|GetsyncedFace))) 1.0)
          (if (> (- (Utilities|Time|GetTimeSeconds) (Variables|Move|GetsyncedTime)) 0.1)
            (CallFunction|SendSyncedMove 1 (LocalVariables|Getlocalstate))
            (return))))
      (:then_3
        (if (> (Variables|Move|GetSpeed) 0.0)
          (if (> (- (Utilities|Time|GetTimeSeconds) (Variables|Move|GetsyncedTime)) 0.1)
            (if (> (Math|Vector|VectorLength (- (Variables|Move|GetsyncedPos) (Transformation|GetActorLocation))) 5.0)
              (CallFunction|SendSyncedMove 2 (LocalVariables|Getlocalstate)))))))))

(fn SendSyncedMove
  (params (kind :type Integer) (state :type Integer))
  (bind _charactermovement (Variables|Character|GetCharacterMovement))
  (bind _maxwalkspeed (Variables|/Script/Engine.CharacterMovementComponent|GetMaxWalkSpeed _charactermovement))
  (LocalVariables|SetLocalKind kind)
  (Variables|Move|SetsyncedState state)
  (Variables|Move|SetsyncedFace (.yaw (Transformation|GetActorRotation)))
  (Variables|Move|SetsyncedPos (Transformation|GetActorLocation))
  (Variables|Move|SetsyncedTime (Utilities|Time|GetTimeSeconds))
  (Utilities|FlowControl|Sequence
    (:then_0
      ;[1 1 1] 预测移动程度，因为0.1秒发一次，而速度为6米/s，所以最多移动60cm，即÷10。Timetemp记录的是speed=0最后时刻，按下移动时间小于0.25时就将移动值设置为30（防止快速只按一下或者起步）
      (LocalVariables|SetLocalSpeed (Variables|Move|GetSpeed))
      (if (< (- (Utilities|Time|GetTimeSeconds) (Variables|Move|GetsyncedTimeTemp)) 0.25)
        (LocalVariables|SetLocalValue (/ _maxwalkspeed 2e+01))
        (else
          (LocalVariables|SetLocalValue (/ _maxwalkspeed 1e+01)))))
    (:then_1
      ;[1 1 1] 预测位移距离
      (if (> (Variables|Move|GetSpeed) 0.0)
        (LocalVariables|SetLocalTargetPos (+ (Transformation|GetActorLocation) (* (Transformation|GetActorForwardVector) (LocalVariables|GetLocalValue))))
        (else
          (LocalVariables|SetLocalTargetPos (Transformation|GetActorLocation)))))
    (:then_2
      ;[1 1 1] 判断障碍物
      (if (CallFunction|IsMoveTrace)
        (LocalVariables|SetLocalTargetPos (Transformation|GetActorLocation))
        (elif (> (LocalVariables|GetLocalKind) 0)
          (LocalVariables|SetLocalSpeed (Variables|/Script/Engine.CharacterMovementComponent|GetMaxWalkSpeed (Variables|Character|GetCharacterMovement))))))
    (:then_3
      (Class|BlueprintFunction|SendMove (Variables|Move|GetsyncedFace) (LocalVariables|GetLocalSpeed) (Variables|Move|GetsyncedPos) (LocalVariables|GetLocalTargetPos)))))

(fn IsMoveTrace
  (bind _returnvalue (Transformation|GetActorLocation))
  ;[1 1 1] 从当前位置到预测位置间有没有障碍物，有就返回T，否则F
  (LocalVariables|SetLocalPos _returnvalue)
  (LocalVariables|SetLocalTargetPos (+ _returnvalue (* (Transformation|GetActorForwardVector) (/ (Variables|/Script/Engine.CharacterMovementComponent|GetMaxWalkSpeed (Variables|Character|GetCharacterMovement)) 1e+01))))
  (bind _returnvalue_2 (Collision|LineTraceForObjects (LocalVariables|GetLocalPos) (LocalVariables|GetLocalTargetPos) (Utilities|Array|MakeArray "ObjectTypeQuery1" "ObjectTypeQuery2") false 0 "None"))
  (return _returnvalue_2))

(fn OnBackPosCommand
  (params (childcmd :type Integer) (pos :type Vector :default "0, 0, 0"))
  (if (== childcmd 3000)
    (Transformation|SetActorLocation pos false false)
    (return false)
    (else
      (Development|PrintString (Utilities|String|Append "移动错误：" (Utilities|String|ToString(Integer) childcmd))))))

(fn UserSkillErrBP
  (params (Err :type Integer))
  (LocalVariables|SetLocalErr Err)
  (if (not (== (LocalVariables|GetLocalErr) 0))
    (Class|MyCharacterBase|ResetAttack)
    (Default|UpdaErrorInfo (Variables|Default|GetMyGameInstance) 3000 (LocalVariables|GetLocalErr))
    (bind _asbp_game_mode (Utilities|Casting|CastToBP_GameMode (Game|GetGameMode)))
    (Utilities|IsValid _asbp_game_mode)))

(fn UseSkillBP
  (LocalVariables|SetLocalAtk (.lock_Atk (Utilities|Struct|BreakUSER_TEMP (.tmp (Utilities|Struct|BreakUSER_ROLE_BASE (Class|BlueprintFunction|MyUserData))))))
  (Utilities|FlowControl|Sequence
    (:then_0
      (if (< (Variables|Default|GetLocalSkillIndex) 10)
        (bind _output_get (LocalVariables|SetLocalSkill (Utilities|Array|Get(acopy) (Utilities|Struct|BreakROLE_STAND_SKILL (.myskill (Utilities|Struct|BreakROLE_STAND (.stand (Utilities|Struct|BreakUSER_ROLE_BASE (Class|BlueprintFunction|MyUserData)))))) (Variables|Default|GetLocalSkillIndex))))
        (bind _returnvalue (Class|BlueprintFunction|GetSkillScriptDistance (.id (Utilities|Struct|BreakROLE_STAND_SKILL_BASE _output_get)) (Math|Conversions|ToInteger(Byte) (.level (Utilities|Struct|BreakROLE_STAND_SKILL_BASE _output_get)))))
        (LocalVariables|SetLocalDistance _returnvalue)
        (switch string (Utilities|String|ToString(Integer) (.id (Utilities|Struct|BreakROLE_STAND_SKILL_BASE _output_get)))
          (:1006
            (if (.IsTrace (CallFunction|IsSkillMoveTrace (Math|Conversions|ToFloat(Integer) (LocalVariables|GetLocalDistance))))
              (LocalVariables|SetLocalDistance (Math|Float|Truncate (- (Math|Vector|VectorLength (- (Transformation|GetActorLocation) (.Location (Collision|BreakHitResult (.OutHit (CallFunction|IsSkillMoveTrace (Math|Conversions|ToFloat(Integer) (LocalVariables|GetLocalDistance)))))))) 5e+01))))))
        (else
          (return 0))))
    (:then_1
      (switch Utilities|FlowControl|Switch|SwitchonE_NODE_TYPE (Utilities|Enum|ByteToEnumE_NODE_TYPE (.lock_Type (Utilities|Struct|BreakLOCK_ATK_DATA (LocalVariables|GetLocalAtk))))
        (:N_FREE
          (Development|PrintString (Utilities|String|ToString(Float) (Math|Conversions|ToFloat(Integer) (LocalVariables|GetLocalDistance))) true true "(R=1.000000,G=0.136410,B=0.056729,A=1.000000)")
          (Class|MyCharacterBase|SetLockTarget "N_FREE" -1 (+ (Transformation|GetActorLocation) (* (Math|Vector|Normalize (Transformation|GetActorForwardVector)) (Math|Conversions|ToFloat(Integer) (LocalVariables|GetLocalDistance))))))
        (:N_ROLE
          (bind _returnvalue_2 (Class|BlueprintFunction|FindUserView (.lock_SkillID (Utilities|Struct|BreakLOCK_ATK_DATA (LocalVariables|GetLocalAtk)))))
          (bind _asother_character (Utilities|Casting|CastToOtherCharacter _returnvalue_2))
          (Class|MyCharacterBase|SetLockTarget "N_ROLE" (.lock_SkillID (Utilities|Struct|BreakLOCK_ATK_DATA (LocalVariables|GetLocalAtk))) (Transformation|GetActorLocation _asother_character)))))
    (:then_2
      (bind _returnvalue_3 (Class|MyCharacterBase|IsUseSkill (Variables|Default|GetLocalSkillIndex)))
      (bind _output_get_2 (LocalVariables|SetLocalErr _returnvalue_3))
      (CallFunction|UserSkillErrBP _output_get_2)
      (switch string (Utilities|String|ToString(Integer) (LocalVariables|GetLocalErr))
        (:0
          (Class|MyCharacterBase|SendSkill (Variables|Default|GetLocalSkillIndex)))
        (:5007
          (Variables|Default|SetIsFollowATK_b true)
          (Default|SetFollowATK (Variables|Default|GetMyPlayerController)))))))

(fn OnSkillCommandErr
  (params (err :type Integer))
  (CallFunction|UserSkillErrBP err)
  (return false))

(fn OnSkillCommandPlay
  (CallFunction|EventPlaySkill)
  (return false))

(fn IsSkillMoveTrace
  (params (Distance :type Float%20%28single-precision%29))
  (bind _returnvalue (Transformation|GetActorLocation))
  (LocalVariables|SetLocalPos _returnvalue)
  (LocalVariables|SetLocalTPos (+ _returnvalue (* (Math|Vector|Normalize (Transformation|GetActorForwardVector)) Distance)))
  (bind _outactors (Actor|GetAllActorsOfClass "/Script/Engine.Pawn"))
  (bind (_outhit _returnvalue_2) (Collision|LineTraceForObjects (+ (LocalVariables|GetLocalPos) "0, 0,20.000000") (+ (LocalVariables|GetLocalTPos) "0, 0,20.000000") (Utilities|Array|MakeArray "ObjectTypeQuery1" "ObjectTypeQuery2") false _outactors "Persistent" true "(R=1.000000,G=0.000000,B=0.000000,A=1.000000)" "(R=0.000000,G=1.000000,B=0.000000,A=1.000000)" 1e+02))
  (return _returnvalue_2 _outhit))

(fn UpdateFollowATK
  (if (Variables|Default|GetIsFollowATK_b)
    (if (Class|CharacterBase|IsMove true)
      (switch int (Class|MyCharacterBase|IsFollowAtk (Variables|Default|GetLocalSkillIndex))
        (:0
          ;[1 1 1] 自动导航到能攻击了
          (Default|StopAIPath (Variables|Default|GetMyPlayerController))
          ;[1 0.007701 0] USERSKILL
          (CallFunction|UseSkillBP))
        (:1
          ;[1 1 1] 出错了
          (Variables|Default|SetIsFollowATK_b false :!label _label)
          (Default|StopAIPath (Variables|Default|GetMyPlayerController)))
        (:2
          (goto _label))
        (:3
          (goto _label))
        (:4
          (goto _label))
        (:5
          ;[1 1 1] 距离还是不够
          (Default|SetFollowATK (Variables|Default|GetMyPlayerController))))
      (else
        (Default|StopAIPath (Variables|Default|GetMyPlayerController))))))

(fn OnBuffCommandPlay
  (params (id :type Integer) (runningtime :type Integer))
  (LocalVariables|Setlocalbuffid id)
  (LocalVariables|Setlocalrunningtime runningtime)
  (LocalVariables|SetLocalBuff (.Value (Utilities|Map|Find (Variables|Default|Getbuff_run) (LocalVariables|Getlocalbuffid))))
  (switch int (LocalVariables|Getlocalrunningtime)
    (:Default
      (Utilities|IsValid (LocalVariables|GetLocalBuff)
        (:Is%20Not%20Valid
          (bind _returnvalue (Game|SpawnActorfromClass "/Game/BuffandSkill/Role_Buff.Role_Buff_C" (Math|Transform|MakeTransform "0, 0, 0" "0, 0, 0" "1,1,1") "Undefined" self 0))
          (bind _output_get (LocalVariables|SetLocalBuff _returnvalue))
          (Transformation|AttachActorToActor _output_get self "None" "KeepRelative" "KeepRelative" "KeepRelative" true)
          (Default|SetBuff (LocalVariables|GetLocalBuff) (LocalVariables|Getlocalbuffid))
          (Utilities|Map|Add (Variables|Default|Getbuff_run) (LocalVariables|Getlocalbuffid) (LocalVariables|GetLocalBuff)))))
    (:0
      (Utilities|Map|Remove (Variables|Default|Getbuff_run) (LocalVariables|Getlocalbuffid))
      (Actor|DestroyActor (LocalVariables|GetLocalBuff)))))

(fn OnCommandLevel
  (params (level :type Integer))
  (return false))

(fn OnCommandDead
  (CallFunction|EventPlayDead)
  (return false))

(fn OnRebornCommandPlay
  (params (err :type Integer) (pos :type Vector :default "0, 0, 0"))
  (switch int err
    (:Default
      (Default|UpdaErrorInfo (Variables|Default|GetMyGameInstance) 4100 err "复活失败！"))
    (:0
      (Transformation|SetActorLocation pos false false)
      (bind _asab_my_animtion (Utilities|Casting|CastToAB_MyAnimtion (Components|SkeletalMesh|GetAnimInstance (Variables|Character|GetMesh))))
      (Variables|/Game/Character/MyCharacter/AB_MyAnimtion.AB_MyAnimtion_C|SetisDead _asab_my_animtion false)
      (CallFunction|SetRebornUI false)
      (return false))))

(fn SetRebornUI
  (params (IsCreate :type Boolean))
  (if IsCreate
    (Utilities|IsValid (Variables|Default|GetRebornUI)
      (:Is%20Not%20Valid
        (bind _returnvalue (UserInterface|CreateWidget "/Game/UI/GameUI/RebornUI.RebornUI_C"))
        (bind _output_get (Variables|Default|SetRebornUI _returnvalue))
        (UserInterface|Viewport|AddtoViewport _output_get 0)
        (Variables|/Script/Engine.PlayerController|SetbShowMouseCursor (Game|GetPlayerController 0) true)))
    (else
      (Utilities|IsValid (Variables|Default|GetRebornUI)
        (:Is%20Valid
          (Widget|RemovefromParent (Variables|Default|GetRebornUI))
          (Variables|Default|SetRebornUI 0)
          (Variables|/Script/Engine.PlayerController|SetbShowMouseCursor (Game|GetPlayerController 0) false))))))

(fn OnSkillCommandColdTime
  (params (skillid :type Integer) (value :type Float%20%28single-precision%29))
  (bind _skillui (Variables|Default|GetSkillUI))
  (Utilities|IsValid _skillui
    (:Is%20Valid
      (Default|SetColdTime _skillui skillid value))))

(fn OnSkillCommandHP
  (params (curhp :type Integer) (atk :type Integer)))