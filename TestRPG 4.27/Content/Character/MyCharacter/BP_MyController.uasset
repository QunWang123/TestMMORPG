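; Player controller that handles chat, bag and item pickup input, relaying HP, chat and drop updates to BP_GameHUD.
; Nearby drops are tracked in a map plus index array that mirrors HUD slots; E sends a pickup request for the first.
; Helpers path to the locked player for follow-attack and stop that movement.
; ClickMouseLeft traces for range-checked drop pickup, but its event-graph call and its targeting and click-to-move branches are disconnected.
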(event EventBeginPlay
  (bind _asbp_my_character (Utilities|Casting|CastToBP_MyCharacter (Pawn|GetControlledPawn)))
  (Variables|Default|SetmyPawn _asbp_my_character)
  (bind _asbp_game_hud (Utilities|Casting|CastToBP_GameHUD (HUD|GetHUD)))
  (Variables|Default|SetmyGameHUD _asbp_game_hud))

(event EventTick
  (params (DeltaSeconds :type Float%20%28single-precision%29)))

(event Input|ActionEvents|InputActionBag
  (params (Key :type Key%20Structure :default "None"))
  (:Released
    (Default|ShowBagWidget (Variables|Default|GetmyGameHUD))))

(event Input|KeyboardEvents|Enter
  (params (Key :type Key%20Structure :default "None"))
  (:Released
    (Utilities|FlowControl|FlipFlop
      (:A
        (Variables|Default|SetbShowMouseCursor true)
        (bind _mygamehud (Variables|Default|GetmyGameHUD)
          (:then
            (Default|ShowChatUI _mygamehud "Visible")
            (Input|SetInputModeGameandUI self (Variables|/Game/GameMode/BP_GameHUD.BP_GameHUD_C|GetMainUI (Variables|Default|GetmyGameHUD)) "DoNotLock" true))
          (:else)))
      (:B
        (Variables|Default|SetbShowMouseCursor false)
        (bind _mygamehud_2 (Variables|Default|GetmyGameHUD)
          (:then
            (Default|ShowChatUI _mygamehud_2 "Hidden")
            (Input|SetInputModeGameandUI self 0 "DoNotLock" true))
          (:else))))))

(event Input|MouseEvents|LeftMouseButton
  (params (Key :type Key%20Structure :default "None")))

(event Input|MouseEvents|RightMouseButton
  (params (Key :type Key%20Structure :default "None")))

(event Input|KeyboardEvents|E
  (params (Key :type Key%20Structure :default "None"))
  (bind _itemlistmap (Variables|Default|GetItemListMap))
  (bind _itemlistindex (Variables|Default|GetItemListIndex))
  (bind _output (Utilities|Array|Get(acopy) _itemlistindex))
  (bind (_value _returnvalue) (Utilities|Map|Find _itemlistmap _output))
  (:Released
    (if (> (Utilities|Array|Length (Variables|Default|GetItemListIndex)) 0)
      (if _returnvalue
        (Class|BlueprintFunction|SendGetDrop _output _value)
        (else
          (Utilities|Array|RemoveIndex (Variables|Default|GetItemListIndex)))))))

(fn ConstructionScript)

(fn ClickMouseLeft
  (bind _self self)
  (bind _hitresult (Game|Player|GetHitResultUnderCursorbyChannel _self "TraceTypeQuery1" true))
  (bind (_bblockinghit _binitialoverlap _time _distance _location _impactpoint) (Collision|BreakHitResult _hitresult))
  (bind (_x _y _z) (Math|Vector|BreakVector _impactpoint))
  (LocalVariables|Setlocal_Location _location)
  (bind _outhit (Collision|LineTraceForObjects (Math|Vector|MakeVector _x _y (- _z 2e+03)) (Math|Vector|MakeVector _x _y (+ _z 2e+03)) (Utilities|Array|MakeArray "ObjectTypeQuery3" "ObjectTypeQuery2") false 0 "Persistent" true "(R=0.817338,G=0.022970,B=1.000000,A=1.000000)" "(R=0.000000,G=1.000000,B=0.000000,A=1.000000)" 99.0))
  (bind _output_get (LocalVariables|SetSelectActor (.HitActor (Collision|BreakHitResult _outhit))))
  (bind _asbp_drop (Utilities|Casting|CastToBP_Drop (LocalVariables|GetSelectActor)))
  (if (< (Transformation|GetDistanceTo (Variables|Default|GetmyPawn) _asbp_drop) 3e+02)
    (Class|BlueprintFunction|SendGetDrop (.dropindex (Utilities|Struct|BreakDROP_BASE (Variables|/Game/Item/Drop/BP_Drop.BP_Drop_C|GetItemData _asbp_drop))) (.dropid (Utilities|Struct|BreakDROP_BASE (Variables|/Game/Item/Drop/BP_Drop.BP_Drop_C|GetItemData _asbp_drop))))
    (else
      ;[1 1 1] 没有锁定目标
      (Development|PrintString "距离掉落过远"))))

(fn StopAIPath
  (if (Variables|Default|GetisAIPath)
    (Variables|Default|SetisAIPath false)
    (AI|Navigation|StopMovement)))

(fn SetFollowATK
  (bind _returnvalue (Class|BlueprintFunction|MyUserData))
  (bind _tmp (Utilities|Struct|BreakUSER_ROLE_BASE _returnvalue))
  (bind _lock_atk (Utilities|Struct|BreakUSER_TEMP _tmp))
  (bind (_lock_skillid _lock_type _lock_index) (Utilities|Struct|BreakLOCK_ATK_DATA _lock_atk))
  (if (Utilities|IsValid (Variables|Default|GetmyPawn))
    (switch Utilities|FlowControl|Switch|SwitchonE_NODE_TYPE (Utilities|Enum|ByteToEnumE_NODE_TYPE _lock_type)
      (:N_ROLE
        (bind _returnvalue_2 (Class|BlueprintFunction|FindUserView _lock_index))
        (bind _asother_character (Utilities|Casting|CastToOtherCharacter _returnvalue_2))
        (AI|Navigation|SimpleMovetoActor self _asother_character)
        (Variables|Default|SetisAIPath true)))))

(fn AddItemtoViewport
  (params (ItemIndex :type Integer) (ItemID :type Integer))
  (bind _itemlistmap (Variables|Default|GetItemListMap))
  (bind _mygamehud (Variables|Default|GetmyGameHUD)
    (:then
      (if (not (.ReturnValue (Utilities|Map|Find _itemlistmap ItemIndex)))
        (Utilities|Map|Add _itemlistmap ItemIndex ItemID)
        (Utilities|Array|Add (Variables|Default|GetItemListIndex) ItemIndex)
        (Default|AddItemSlot _mygamehud ItemIndex ItemID)))
    (:else)))

(fn UpdateMainCharacterHP
  (params (CurHP :type Float%20%28single-precision%29) (Atk :type Integer))
  (bind _mygamehud (Variables|Default|GetmyGameHUD)
    (:then
      (Default|UpdateMainCharacterHP _mygamehud CurHP Atk))
    (:else)))

(fn RemoveItemfromViewport
  (params (ItemIndex :type Integer))
  (bind _itemlistmap (Variables|Default|GetItemListMap))
  (bind _mygamehud (Variables|Default|GetmyGameHUD)
    (:then
      (if (.ReturnValue (Utilities|Map|Find _itemlistmap ItemIndex))
        (Utilities|Map|Remove _itemlistmap ItemIndex)
        (Utilities|FlowControl|Sequence
          (:then_0
            (Default|RemoveItemSlot _mygamehud ItemIndex))
          (:then_1
            (Utilities|Array|RemoveIndex (Variables|Default|GetItemListIndex))))))
    (:else)))

(fn AddChatText
  (params (InText :type String))
  (bind _mygamehud (Variables|Default|GetmyGameHUD)
    (:then
      (Default|AddChatText _mygamehud InText))
    (:else)))